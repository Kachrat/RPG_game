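; Player attack component that runs a scythe combo from the attack input, gated by CanAttack.
; SytheAttack buffers presses made while IsAttacking, otherwise selects an attack by AttackIndex; only the first, a delayed montage behind a DoOnce, is wired.
; SytheAttackCombo consumes the buffered press to re-enter that selection, or calls StopCombo to reset the state.
; Nothing here sets IsAttacking true or calls SytheAttackCombo.
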(event `EnhancedInput|/Game/Character/BP_PlayerCharacter/Input/Actions/IA_Attack`
  (params (ActionValue :type Boolean) (ElapsedSeconds :type "Float (double-precision)") (TriggeredSeconds :type "Float (double-precision)") (InputAction :type "InputAction Object Reference" :default "/Game/Character/BP_PlayerCharacter/Input/Actions/IA_Attack.IA_Attack"))
  ;[0.07812 0.07812 0.07812] Attack Input
  (:`Started`
    (if (`self.can Attack?`)
      (`self.Sythe Attack`))))

(event `Attack 1`
  ;[0.07812 0.07812 0.07812] Attack 1
  (`/Engine/EditorBlueprintResources/StandardMacros.DoOnce` false :!label _label
    (:`Completed`
      (`KismetSystemLibrary.Delay` 0.1)
      (`|PlayMontage` null
        (:`then`
          (set `self.Attack Index` 1)
          (goto _label :!via `Reset`))))))

(event `Sythe Attack`
  ;[0.07812 0.07812 0.07812] Sythe Attack
  (if (`self.is Attacking?`)
    (set `self.save Attack?` true)
    (else
      (set `self.save Attack?` false)
      (switch `int` (`self.Attack Index`) :!label _label_2
        (:`0`
          (`self.Attack 1`))))))

(event `Sythe Attack Combo`
  ;[0.07812 0.07812 0.07812] Combo Continue
  (if (`self.save Attack?`)
    (set `self.save Attack?` false)
    (goto _label_2)
    (else
      (`self.Stop Combo`))))

(event `Stop Combo`
  ;[0.07812 0.07812 0.07812] Stop Combo / Attack
  (set `self.is Attacking?` false)
  (set `self.Attack Index` 0))